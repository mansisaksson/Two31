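; Spawner actor that continuously emits BloodParticleBall actors from its own position to produce a blood spray.
; BeginPlay starts a self-restarting 0.01-second Delay loop with no stop condition, spawning one ball per pass.
; Each ball takes the spawner's location and scale with a random rotation, then receives the BloodSplat1 decal and a randomized lifetime and speed.
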(event EventBeginPlay
  (bind _returnvalue (Transformation|GetActorTransform))
  (bind (_location _rotation _scale) (Math|Transform|BreakTransform _returnvalue))
  (Utilities|FlowControl|Delay 0.01 :!label _label)
  (Utilities|FlowControl|Sequence
    (:then_0
      (goto _label))
    (:then_1
      (bind _returnvalue_2 (Game|SpawnActorfromClass "/Script/Two31.BloodParticleBall" (Math|Transform|MakeTransform _location (Math|Random|RandomRotator true) _scale) "Undefined" 0 0))
      (Variables|/Script/Two31.BloodParticleBall|SetDecal _returnvalue_2 "/Game/Assets/Materials/Decal/BloodSplat1.BloodSplat1")
      (Variables|/Script/Two31.BloodParticleBall|SetLifetimeDestroy _returnvalue_2 (Math|Conversions|ToFloat(Integer) (Math|Random|RandomInteger 10)))
      (Variables|/Script/Two31.BloodParticleBall|SetSpeed _returnvalue_2 (Math|Conversions|ToFloat(Integer) (* (Math|Random|RandomInteger 30) 100))))))

(event EventActorBeginOverlap
  (params (OtherActor :type Actor%20Object%20Reference)))

(event EventTick
  (params (DeltaSeconds :type Float%20%28single-precision%29)))

(fn ConstructionScript)