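; BP_ElevatorMusic is a trigger zone that switches elevator music on while the player is inside its box.
; Player overlap activates the Music component and deactivates it on exit.
; The follow-on FMOD snapshot playback sits behind a cast with no input, so it cannot play.
; BeginPlay caches the first BP_MusicActor, which goes unused here, and unconnected pause and event-playback nodes remain.
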(event OnComponentBeginOverlap(Box)
  (params (OtherActor :type Actor%20Object%20Reference) (OtherComp :type Primitive%20Component%20Object%20Reference) (OtherBodyIndex :type Integer) (bFromSweep :type Boolean) (SweepResult :type Hit%20Result%20Structure%20%28by%20ref%29))
  (Utilities|Casting|CastToPlayerCharacter OtherActor)
  (Components|Activation|Activate (Variables|Default|GetMusic) false)
  (bind _asfmodsnapshot (Utilities|Casting|CastToFMODSnapshot))
  (Class|FMODBlueprintStatics|PlayEventatLocation _asfmodsnapshot (Math|Conversions|ToTransform(Vector) (Transformation|GetActorLocation))))

(event OnComponentEndOverlap(Box)
  (params (OtherActor :type Actor%20Object%20Reference) (OtherComp :type Primitive%20Component%20Object%20Reference) (OtherBodyIndex :type Integer))
  (Utilities|Casting|CastToPlayerCharacter OtherActor)
  (Components|Activation|Deactivate (Variables|Default|GetMusic)))

(event EventBeginPlay
  ;[1 1 1] Disisnotgood
  (bind _outactors (Actor|GetAllActorsOfClass "/Game/Blueprints/Music/BP_MusicActor.BP_MusicActor_C"))
  (Variables|Default|SetMusicActor (Utilities|Array|Get(acopy) _outactors)))

(fn ConstructionScript)