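; BP_StingerBall is a trigger actor that fires a music stinger when the player enters it.
; On BeginPlay it caches the first BP_MusicActor found in the level.
; When a PlayerCharacter begins overlapping TriggerBox, it sets the "Stinger" parameter on that actor's Music to 1 and prints a debug string.
; Nothing here resets the parameter, and a Music Stop node is left unconnected.
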(event OnComponentBeginOverlap(TriggerBox)
  (params (OtherActor :type Actor%20Object%20Reference) (OtherComp :type Primitive%20Component%20Object%20Reference) (OtherBodyIndex :type Integer) (bFromSweep :type Boolean) (SweepResult :type Hit%20Result%20Structure%20%28by%20ref%29))
  ;[1 1 1] StingerBollen
  (Utilities|Casting|CastToPlayerCharacter OtherActor)
  (Class|FMODAudioComponent|SetParameter (Variables|/Game/Blueprints/Music/BP_MusicActor.BP_MusicActor_C|GetMusic (Variables|Default|GetMusicActor)) "Stinger" 1.0)
  (Development|PrintString "Urgrgrg"))

(event EventBeginPlay
  (bind _outactors (Actor|GetAllActorsOfClass "/Game/Blueprints/Music/BP_MusicActor.BP_MusicActor_C"))
  (Variables|Default|SetMusicActor (Utilities|Array|Get(acopy) _outactors)))

(fn ConstructionScript)