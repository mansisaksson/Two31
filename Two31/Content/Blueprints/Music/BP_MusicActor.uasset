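; Music manager actor that plays the game's music and switches its battle layer based on how many enemies are triggered.
; BeginPlay calls ClearBuffer and starts the Music component.
; Tick polls the Triggered enemy count, setting the Battle parameter on above three and off only at zero, so the gap acts as hysteresis.
; Snapshot playback, debug printing and an Elevator parameter are left unconnected.
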(event EventTick
  (params (DeltaSeconds :type Float%20%28single-precision%29))
  (Utilities|FlowControl|Sequence
    (:then_0
      ;[1 1 1] Start Battle Music
      (bind _returnvalue (Class|MusicManager|GetNumberOfEnemiesinState "Triggered"))
      (if (> _returnvalue 3)
        (Class|FMODAudioComponent|SetParameter (Variables|Default|GetMusic) "Battle" 1.0)))
    (:then_1
      ;[1 1 1] Stop Battle Music
      (bind _returnvalue_2 (Class|MusicManager|GetNumberOfEnemiesinState "Triggered"))
      (if (== _returnvalue_2 0)
        (Class|FMODAudioComponent|SetParameter (Variables|Default|GetMusic) "Battle" 0.0)))
    (:then_2
      (bind _returnvalue_3 (Class|MusicManager|GetNumberOfEnemiesinState "Triggered")))))

(event EventBeginPlay
  (Class|MusicManager|ClearBuffer)
  (Class|FMODAudioComponent|Play (Variables|Default|GetMusic)))

(event EventActorBeginOverlap
  (params (OtherActor :type Actor%20Object%20Reference)))

(fn ConstructionScript)