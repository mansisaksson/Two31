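; Elevator room music actor that plays an FMOD audio component as the player enters two nested trigger volumes.
; The outer box starts Music02 with the Elevator parameter off; the inner room switches to HizzJazz with it on, turning it off on exit.
; Leaving the outer box does nothing.
; Tick rebinds to the player character's stop-music event every frame, so the music stops on death.
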(event OnComponentEndOverlap(TriggerBox)
  (params (OtherActor :type Actor%20Object%20Reference) (OtherComp :type Primitive%20Component%20Object%20Reference) (OtherBodyIndex :type Integer))
  ;[1 1 1] Yttre Boxen
  (Utilities|Casting|CastToPlayerCharacter OtherActor))

(event OnComponentBeginOverlap(InnerRoom)
  (params (OtherActor :type Actor%20Object%20Reference) (OtherComp :type Primitive%20Component%20Object%20Reference) (OtherBodyIndex :type Integer) (bFromSweep :type Boolean) (SweepResult :type Hit%20Result%20Structure%20%28by%20ref%29))
  (bind _music02 (Variables|Default|GetMusic02))
  ;[1 1 1] Innnre Boxen
  (Utilities|Casting|CastToPlayerCharacter OtherActor)
  (Class|FMODAudioComponent|SetEvent _music02 "/Game/FMOD/Events/Music/HizzJazz.HizzJazz")
  (Class|FMODAudioComponent|Play _music02)
  (Class|FMODAudioComponent|SetParameter _music02 "Elevator" 1.0))

(event OnComponentEndOverlap(InnerRoom)
  (params (OtherActor :type Actor%20Object%20Reference) (OtherComp :type Primitive%20Component%20Object%20Reference) (OtherBodyIndex :type Integer))
  ;[1 1 1] Innnre Boxen
  (Utilities|Casting|CastToPlayerCharacter OtherActor)
  (Class|FMODAudioComponent|SetParameter (Variables|Default|GetMusic02) "Elevator" 0.0))

(event OnComponentBeginOverlap(TriggerBox)
  (params (OtherActor :type Actor%20Object%20Reference) (OtherComp :type Primitive%20Component%20Object%20Reference) (OtherBodyIndex :type Integer) (bFromSweep :type Boolean) (SweepResult :type Hit%20Result%20Structure%20%28by%20ref%29))
  (bind _music02 (Variables|Default|GetMusic02))
  ;[1 1 1] Yttre Boxen
  (Utilities|Casting|CastToPlayerCharacter OtherActor)
  (Class|FMODAudioComponent|Play _music02)
  (Class|FMODAudioComponent|SetParameter _music02 "Elevator" 0.0))

(event Custom|MusicStop
  ;[1 1 1] Stop on player death
  (Class|FMODAudioComponent|Stop (Variables|Default|GetMusic02)))

(event EventTick
  (params (DeltaSeconds :type Float%20%28single-precision%29))
  ;[1 1 1] Stop on player death
  (bind _asbp_player_character (Utilities|Casting|CastToBP_PlayerCharacter (Game|GetPlayerCharacter 0)))
  (EventDispatchers|BindEventtoStopMusic _asbp_player_character (delegate Custom|MusicStop)))

(event EventBeginPlay)

(event EventActorBeginOverlap
  (params (OtherActor :type Actor%20Object%20Reference)))

(event EventTick
  (params (DeltaSeconds :type Float%20%28single-precision%29)))

(fn ConstructionScript)