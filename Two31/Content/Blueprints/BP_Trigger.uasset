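; BP_Trigger is a limited-use trigger volume that sends nearby imps toward the player on entry.
; The construction script sizes the box from Size.
; Each player overlap while Amount is positive decrements it and issues SimpleMoveToLocation to every BP_ImpCharacter inside the Sphere, targeting the player's position at that moment.
; An overlap after Amount runs out only sets Complete.
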(event OnComponentBeginOverlap(TriggerBox)
  (params (OtherActor :type Actor%20Object%20Reference) (OtherComp :type Primitive%20Component%20Object%20Reference) (OtherBodyIndex :type Integer) (bFromSweep :type Boolean) (SweepResult :type Hit%20Result%20Structure%20%28by%20ref%29))
  ;[1 1 1] Trigger and Action
  (bind _asplayer_character (Utilities|Casting|CastToPlayerCharacter OtherActor))
  (if (> (Variables|TriggerBox|GetAmount) 0)
    (Variables|TriggerBox|SetAmount (- (Variables|TriggerBox|GetAmount) 1))
    (for _array_element (Collision|GetOverlappingActors (Variables|Default|GetSphere) "/Game/Blueprints/BP_ImpCharacter.BP_ImpCharacter_C" :!class /Script/Engine.PrimitiveComponent)
      (AI|Navigation|SimpleMovetoLocation (Pawn|GetController (Variables|/Script/Engine.Actor|GetInstigator _array_element)) (Transformation|GetActorLocation _asplayer_character)))
    (else
      (Variables|TriggerBox|SetComplete true))))

(event EventBeginPlay)

(event EventActorBeginOverlap
  (params (OtherActor :type Actor%20Object%20Reference)))

(event EventTick
  (params (DeltaSeconds :type Float%20%28single-precision%29)))

(fn ConstructionScript
  ;[1 1 1] Set Trigger Box Size
  (Components|Box|SetBoxExtent (Variables|Default|GetTriggerBox) (Variables|TriggerBox|GetSize) true))