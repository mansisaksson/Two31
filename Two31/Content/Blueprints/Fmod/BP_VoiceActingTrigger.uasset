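; BP_VoiceActingTrigger is a trigger volume that plays a voice line once when the player character overlaps its box.
; It can optionally require the player to hold a specific item, staying armed until that condition is met.
; On firing, it passes the voice ID and timer to the player, disables itself, and plays the Speaches audio, using the ID as the SpeachSelect parameter to choose the line.
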(event OnComponentBeginOverlap(TriggerBox)
  (params (OtherActor :type Actor%20Object%20Reference) (OtherComp :type Primitive%20Component%20Object%20Reference) (OtherBodyIndex :type Integer) (bFromSweep :type Boolean) (SweepResult :type Hit%20Result%20Structure%20%28by%20ref%29))
  (bind _voiceactingid (Variables|Default|GetVoiceActingID))
  (bind _speaches (Variables|Default|GetSpeaches))
  (bind _speaches_2 (Variables|Default|GetSpeaches))
  (bind _voiceactingid_2 (Variables|Default|GetVoiceActingID))
  (bind _asplayer_character (Utilities|Casting|CastToPlayerCharacter OtherActor))
  (if (Variables|Default|GetRequiresItem)
    (if (Class|PlayerCharacter|PlayerHasItem _asplayer_character (Variables|Default|GetRequiredItemID))
      (if (Variables|Default|GetCanBeActivated)
        (Class|PlayerCharacter|AddVoiceActingID _asplayer_character _voiceactingid_2)
        (Class|PlayerCharacter|AddVoiceActingTimer _asplayer_character (Variables|Default|GetTimer))
        (Variables|Default|SetCanBeActivated false)
        (Class|FMODAudioComponent|SetParameter _speaches_2 "SpeachSelect" (Math|Conversions|ToFloat(Integer) _voiceactingid_2))
        (Class|FMODAudioComponent|Play _speaches_2)))
    (elif (Variables|Default|GetCanBeActivated)
      (Class|PlayerCharacter|AddVoiceActingID _asplayer_character _voiceactingid)
      (Class|PlayerCharacter|AddVoiceActingTimer _asplayer_character (Variables|Default|GetTimer))
      (Variables|Default|SetCanBeActivated false)
      (Class|FMODAudioComponent|SetParameter _speaches "SpeachSelect" (Math|Conversions|ToFloat(Integer) _voiceactingid))
      (Class|FMODAudioComponent|Play _speaches))))

(event EventBeginPlay)

(event EventActorBeginOverlap
  (params (OtherActor :type Actor%20Object%20Reference)))

(event EventTick
  (params (DeltaSeconds :type Float%20%28single-precision%29)))

(fn ConstructionScript)