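; BP_TwoWayTrigger is an AI trigger volume that forces an Imp character to keep moving along a world X or Y axis while inside it.
; On begin overlap, it picks the axis by comparing the signed forward-vector X and Y, without absolute values, then takes that component's sign for the ForceMovement direction.
; On end overlap, it calls StopForcedMovement on the Imp.
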(event OnComponentBeginOverlap(TriggerBox)
  (params (OtherActor :type Actor%20Object%20Reference) (OtherComp :type Primitive%20Component%20Object%20Reference) (OtherBodyIndex :type Integer) (bFromSweep :type Boolean) (SweepResult :type Hit%20Result%20Structure%20%28by%20ref%29))
  ;[0.4341 1 0.4269] Force Movement Continue Direction
  (bind _asbp_imp_character (Utilities|Casting|CastToBP_ImpCharacter OtherActor))
  (if (< (.X (Math|Vector|BreakVector (Transformation|GetActorForwardVector _asbp_imp_character))) (.Y (Math|Vector|BreakVector (Transformation|GetActorForwardVector _asbp_imp_character))))
    (if (< (.Y (Math|Vector|BreakVector (Transformation|GetActorForwardVector _asbp_imp_character))) 0.0)
      (Class|ImpCharacter|ForceMovement _asbp_imp_character "0,-1.000000, 0")
      (else
        (Class|ImpCharacter|ForceMovement _asbp_imp_character "0,1.000000, 0")))
    (elif (< (.X (Math|Vector|BreakVector (Transformation|GetActorForwardVector _asbp_imp_character))) 0.0)
      (Class|ImpCharacter|ForceMovement _asbp_imp_character "-1.000000, 0, 0")
      (else
        (Class|ImpCharacter|ForceMovement _asbp_imp_character "1.000000, 0, 0")))))

(event OnComponentEndOverlap(TriggerBox)
  (params (OtherActor :type Actor%20Object%20Reference) (OtherComp :type Primitive%20Component%20Object%20Reference) (OtherBodyIndex :type Integer))
  ;[1 0.2272 0.189] Stop Forced Movement
  (bind _asbp_imp_character (Utilities|Casting|CastToBP_ImpCharacter OtherActor))
  (Class|ImpCharacter|StopForcedMovement _asbp_imp_character))

(event EventBeginPlay)

(event EventActorBeginOverlap
  (params (OtherActor :type Actor%20Object%20Reference)))

(event EventTick
  (params (DeltaSeconds :type Float%20%28single-precision%29)))

(fn ConstructionScript)