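; BP_SecretTrigger is a trigger volume that marks a secret area for the player to discover.
; On its first Tick it registers itself by increasing the total secret count.
; When a PlayerCharacter first overlaps its TriggerBox, it flags itself found, increments the found-secrets count and shows its SecretText through the player's display text.
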(event OnComponentBeginOverlap(TriggerBox)
  (params (OtherActor :type Actor%20Object%20Reference) (OtherComp :type Primitive%20Component%20Object%20Reference) (OtherBodyIndex :type Integer) (bFromSweep :type Boolean) (SweepResult :type Hit%20Result%20Structure%20%28by%20ref%29))
  (bind _asplayer_character (Utilities|Casting|CastToPlayerCharacter OtherActor))
  (if (not (Variables|Default|GetSecretFound))
    (Variables|Default|SetSecretFound true)
    (Class|StatsPornManager|IncreaseAmountOfSecretsFound)
    (Class|PlayerCharacter|AddDisplayText _asplayer_character (Variables|Default|GetSecretText))))

(event EventBeginPlay)

(event EventActorBeginOverlap
  (params (OtherActor :type Actor%20Object%20Reference)))

(event EventTick
  (params (DeltaSeconds :type Float%20%28single-precision%29))
  (if (Variables|Default|GetFirstTick)
    (Variables|Default|SetFirstTick false)
    (Class|StatsPornManager|IncreaseAmountOfSecrets)))

(fn ConstructionScript)