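; BP_GameCompleteTrigger is a trigger actor that ends the game when the player character overlaps its box.
; On overlap it adds the GameCompleteScreen widget to the viewport and shows the mouse cursor.
; It then disables controller and character input, hides the first-person arms and current weapon, and turns off the character's collision.
; Finally it calls SetLevelCompletionTimer on the player character.
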(event OnComponentBeginOverlap(TriggerBox)
  (params (OtherActor :type Actor%20Object%20Reference) (OtherComp :type Primitive%20Component%20Object%20Reference) (OtherBodyIndex :type Integer) (bFromSweep :type Boolean) (SweepResult :type Hit%20Result%20Structure%20%28by%20ref%29))
  (bind _returnvalue (Game|GetPlayerController 0))
  (bind _asplayer_character (Utilities|Casting|CastToPlayerCharacter OtherActor))
  (Utilities|FlowControl|Sequence
    (:then_0
      ;[1 1 1] Create Widget
      (bind _returnvalue_2 (UserInterface|CreateWidget "/Game/Blueprints/Menu/GameCompleteScreen.GameCompleteScreen_C"))
      (UserInterface|Viewport|AddtoViewport _returnvalue_2 0)
      (Variables|/Script/Engine.PlayerController|SetbShowMouseCursor (Game|GetPlayerController 0) true))
    (:then_1
      ;[1 1 1] Hide Arms + Gun
      (Input|DisableInput _returnvalue _returnvalue)
      (Development|SetHiddeninGame (Class|PlayerCharacter|GetFPMeshArmMesh _asplayer_character) true false)
      (Rendering|SetActorHiddenInGame (Class|PlayerCharacter|GetCurrentWeapon _asplayer_character) true)
      (Collision|SetActorEnableCollision _asplayer_character false))
    (:then_2
      (bind _asplayer_character_2 (Utilities|Casting|CastToPlayerCharacter (Game|GetPlayerCharacter 0)))
      (Class|PlayerCharacter|SetLevelCompletionTimer _asplayer_character_2))))

(event EventBeginPlay)

(event EventActorBeginOverlap
  (params (OtherActor :type Actor%20Object%20Reference)))

(event EventTick
  (params (DeltaSeconds :type Float%20%28single-precision%29)))

(fn ConstructionScript)