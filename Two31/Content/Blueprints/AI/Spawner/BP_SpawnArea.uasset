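; BP_SpawnArea is a placeable spawner that populates a box with enemies or test meshes when the player enters its trigger.
; Each player overlap uses up one of a limited number of spawns and creates a batch sized by NumOfEnemies.
; SpawnSetting selects instanced static meshes or Imp child actor components, placed at random relative positions from a random stream.
; The construction script sizes the spawn box from SpawningArea.
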(event OnComponentBeginOverlap(SpawnTrigger)
  (params (OtherActor :type Actor%20Object%20Reference) (OtherComp :type Primitive%20Component%20Object%20Reference) (OtherBodyIndex :type Integer) (bFromSweep :type Boolean) (SweepResult :type Hit%20Result%20Structure%20%28by%20ref%29))
  (bind _spawnarea (Variables|Default|GetSpawnArea))
  (bind _randomspawnstream (Variables|SpawnSettings|GetRandomSpawnStream))
  (bind _boxextent (Variables|/Script/Engine.BoxComponent|GetBoxExtent _spawnarea))
  (bind _returnvalue (* (.z _boxextent) -1.0))
  (bind _returnvalue_2 (* (.x _boxextent) -1.0))
  (bind _returnvalue_3 (* (.y _boxextent) -1.0))
  (bind _returnvalue_4 (Math|Random|RandomFloatinRangefromStream _returnvalue (.z _boxextent) _randomspawnstream))
  (bind _returnvalue_5 (Math|Random|RandomFloatinRangefromStream _returnvalue_2 (.x _boxextent) _randomspawnstream))
  (bind _returnvalue_6 (Math|Random|RandomFloatinRangefromStream _returnvalue_3 (.y _boxextent) _randomspawnstream))
  (bind _returnvalue_7 (Math|Vector|MakeVector _returnvalue_5 _returnvalue_6 _returnvalue_4))
  ;[1 1 1] SpawnSettings
  (Utilities|Casting|CastToPlayerCharacter OtherActor)
  (if (> (Variables|SpawnSettings|GetAmountOfSpawns) 0)
    (Variables|SpawnSettings|SetAmountOfSpawns (- (Variables|SpawnSettings|GetAmountOfSpawns) 1))
    (switch Utilities|FlowControl|Switch|SwitchonEnum_EnemyTypes (Variables|SpawnSettings|GetSpawnSetting)
      (:NewEnumerator0
        ;[1 1 1] TestBoxes
        (for _index (range 1 (Variables|SpawnSettings|GetNumOfEnemies))
          (Components|InstancedStaticMesh|AddInstance (Variables|Default|GetSourceMesh) (Math|Transform|MakeTransform _returnvalue_7 "0, 0, 0" "1,1,1"))))
      (:NewEnumerator1
        ;[1 1 1] EnemyImp
        (for _index_2 (range 1 (Variables|SpawnSettings|GetNumOfEnemies))
          (AddComponent|AddChildActorComponent false (Math|Transform|MakeTransform _returnvalue_7 "0, 0, 0" "1,1,1")))))))

(event EventBeginPlay)

(event EventActorBeginOverlap
  (params (OtherActor :type Actor%20Object%20Reference)))

(event EventTick
  (params (DeltaSeconds :type Float%20%28single-precision%29)))

(fn ConstructionScript
  (Components|Box|SetBoxExtent (Variables|Default|GetSpawnArea) (Variables|SpawnSettings|GetSpawningArea) true))