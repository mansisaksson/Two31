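; CustomDecal is an actor that, despite its name, currently only probes and visualizes a box volume, with no decal logic in its graphs.
; The construction script scales TriggerBox from the Size variable divided by 100.
; On BeginPlay it runs a box overlap at the root's location using Size as extent, prints each WorldStatic or Destructible actor found, and draws a temporary debug box.
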(event EventBeginPlay
  (Utilities|FlowControl|Sequence
    (:then_0
      (bind _outactors (Class|KismetSystemLibrary|BoxOverlapActorsNEW (Transformation|GetWorldLocation (Variables|Default|GetDefaultSceneRoot)) (Variables|CustomDecal|GetSize) (Utilities|Array|MakeArray "ObjectTypeQuery1" "ObjectTypeQuery6")))
      (for _array_element _outactors
        (Development|PrintString (Utilities|GetDisplayName _array_element))))
    (:then_1
      (Rendering|Debug|DrawDebugBox (Transformation|GetWorldLocation (Variables|Default|GetDefaultSceneRoot)) (Variables|CustomDecal|GetSize) "(R=1.000000,G=0.000000,B=0.789950,A=1.000000)" "0, 0, 0" 1e+01))))

(event EventActorBeginOverlap
  (params (OtherActor :type Actor%20Object%20Reference)))

(event EventTick
  (params (DeltaSeconds :type Float%20%28single-precision%29)))

(fn ConstructionScript
  (Transformation|SetRelativeScale3D (Variables|Default|GetTriggerBox) (/ (Variables|CustomDecal|GetSize) 1e+02)))