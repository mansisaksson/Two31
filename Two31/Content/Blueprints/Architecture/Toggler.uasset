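; Toggler is an actor Blueprint that holds an IsOn flag controlling its own visibility.
; The construction script, TurnOn, TurnOff and SetState pass IsOn straight to SetActorHiddenInGame, so on means hidden in game.
; ToggleState instead flips the flag and sets root visibility to IsOn, propagated to children, so on means visible there.
; GetState returns the flag, and the event graph is empty.
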(event EventBeginPlay)

(event EventActorBeginOverlap
  (params (OtherActor :type Actor%20Object%20Reference)))

(event EventTick
  (params (DeltaSeconds :type Float%20%28single-precision%29)))

(fn ConstructionScript
  (Rendering|SetActorHiddenInGame (Variables|TogglerSetup|GetIsOn)))

(fn Turnon
  (bind _output_get (Variables|TogglerSetup|SetIsOn true))
  (Rendering|SetActorHiddenInGame _output_get))

(fn TurnOff
  (bind _output_get (Variables|TogglerSetup|SetIsOn false))
  (Rendering|SetActorHiddenInGame _output_get))

(fn SetState
  (params (State :type Boolean))
  (bind _output_get (Variables|TogglerSetup|SetIsOn State))
  (Rendering|SetActorHiddenInGame _output_get))

(fn GetState
  (return (Variables|TogglerSetup|GetIsOn)))

(fn ToggleState
  (bind _output_get (Variables|TogglerSetup|SetIsOn (not (Variables|TogglerSetup|GetIsOn))))
  (Rendering|SetVisibility (Variables|Default|GetDefaultSceneRoot) _output_get true))