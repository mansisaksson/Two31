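; Base interactable actor that highlights when the player looks at it and broadcasts OnInteract when Interact is pressed while in sight.
; A looping timer runs UpdateTrace, a multi line trace from the player's eyes on the Visibility channel.
; Hits on itself set IsInSight and toggle the mesh's custom depth.
; Each instance traces and enables input independently, with its mesh set from InteractMesh at construction.
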(event EventBeginPlay
  (Utilities|FlowControl|Sequence
    (:then_0
      (Utilities|Time|SetTimerbyFunctionName self "UpdateTrace" (Variables|InteractableSetup|GetTraceUpdateTime) true))
    (:then_1
      (Input|EnableInput (Game|GetPlayerController 0)))))

(event EventActorBeginOverlap
  (params (OtherActor :type Actor%20Object%20Reference)))

(event EventTick
  (params (DeltaSeconds :type Float%20%28single-precision%29)))

(event Input|ActionEvents|InputActionInteract
  (params (Key :type Key%20Structure :default "AnyKey"))
  (:Pressed
    (if (Variables|Default|GetIsInSight)
      (Default|CallOnInteract))))

(fn ConstructionScript
  (bind _interactmesh (Variables|InteractableSetup|GetInteractMesh))
  (if (not (== _interactmesh 0))
    (Components|StaticMesh|SetStaticMesh (Variables|Default|GetMesh) _interactmesh)))

(fn UpdateTrace
  (bind _returnvalue (Game|GetPlayerCharacter 0))
  (bind (_outlocation _outrotation) (Actor|GetActorEyesViewPoint _returnvalue))
  (Utilities|FlowControl|Sequence
    (:then_0
      (Variables|Default|SetTemp false))
    (:then_1
      (bind _outhits (Class|KismetSystemLibrary|LineTraceMultiNEW _outlocation (+ _outlocation (* (Math|Vector|GetForwardVector _outrotation) (Variables|InteractableSetup|GetInteractableDistance))) "TraceTypeQuery1" false 0 "None" false))
      (for _index (range 0 (Utilities|Array|Length _outhits))
        (if (== self (.HitActor (Collision|BreakHitResult (Utilities|Array|Get(acopy) _outhits _index))))
          (Variables|Default|SetTemp true)))
      (Rendering|SetRenderCustomDepth (Variables|Default|GetMesh) (Variables|Default|GetTemp))
      (Variables|Default|SetIsInSight (Variables|Default|GetTemp)))))