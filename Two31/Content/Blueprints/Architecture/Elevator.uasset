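; Elevator actor that moves its Scene component between floors defined as offsets in a Floors array.
; Construction records the start location, snaps to the first floor and scales timeline speed by AnimationTime.
; Up, down and go-to-floor functions set the target unless the lerp is mid-travel, then fire OnFloorChange.
; That event's timeline lerps between floor positions, then updates the previous floor and calls OnArrival.
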(event Custom|OnFloorChange
  (bind _driver (Timeline|Timeline_0 PlayFromStart)
    (:Update
      (Transformation|SetRelativeLocation (Variables|Default|GetScene) (Math|Vector|Lerp(Vector) (+ (Utilities|Array|Get(acopy) (Variables|ElevatorSetup|GetFloors) (Variables|Default|GetPreviousFloor)) (Variables|Default|GetStartingLocation)) (+ (Utilities|Array|Get(acopy) (Variables|ElevatorSetup|GetFloors) (Variables|Default|GetTargetFloor)) (Variables|Default|GetStartingLocation)) _driver) false false)
      (Variables|Default|SetLerpValue _driver))
    (:Finished
      (Variables|Default|SetPreviousFloor (Variables|Default|GetTargetFloor))
      (Default|CallOnArrival))))

(event EventBeginPlay)

(event EventActorBeginOverlap
  (params (OtherActor :type Actor%20Object%20Reference)))

(event EventTick
  (params (DeltaSeconds :type Float%20%28single-precision%29)))

(fn ConstructionScript
  (Variables|Default|SetStartingLocation (Transformation|GetWorldLocation (Variables|Default|GetScene)))
  (Transformation|SetWorldLocation (Variables|Default|GetScene) (+ (Utilities|Array|Get(acopy) (Variables|ElevatorSetup|GetFloors)) (Variables|Default|GetStartingLocation)) false false)
  (Components|Timeline|SetPlayRate (Variables|Default|GetTimeline_0) (/ 1.0 (Variables|ElevatorSetup|GetAnimationTime))))

(fn MoveFloorUp
  (bind _ismoving (CallFunction|IsMoving))
  (if (not _ismoving)
    (Variables|Default|SetTargetFloor (Math|Integer|Clamp(Integer) (+ (Variables|Default|GetTargetFloor) 1) 0 (- (Utilities|Array|Length (Variables|ElevatorSetup|GetFloors)) 1)))
    (CallFunction|OnFloorChange)))

(fn MoveFloorDown
  (bind _ismoving (CallFunction|IsMoving))
  (if (not _ismoving)
    (Variables|Default|SetTargetFloor (Math|Integer|Clamp(Integer) (- (Variables|Default|GetTargetFloor) 1) 0 (- (Utilities|Array|Length (Variables|ElevatorSetup|GetFloors)) 1)))
    (CallFunction|OnFloorChange)))

(fn MoveFloor
  (params (TargetFloor :type Integer))
  (bind _ismoving (CallFunction|IsMoving))
  (if (and (not _ismoving) (not (== TargetFloor (Variables|Default|GetTargetFloor))))
    (Variables|Default|SetTargetFloor TargetFloor)
    (CallFunction|OnFloorChange)))

(fn IsMoving
  (return (not (or (<= (Variables|Default|GetLerpValue) 0.01) (>= (Variables|Default|GetLerpValue) 0.99)))))

(fn GetCurrentFloor
  (return (Variables|Default|GetTargetFloor)))