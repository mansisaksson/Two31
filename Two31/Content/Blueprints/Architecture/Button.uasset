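; Interactable button actor that checks whether the player is aiming at it when Interact is pressed, with no response to a successful press implemented.
; It enables input for player 0 on BeginPlay, then on each press runs a debug-drawn multi line trace on Visibility from the character's eyes out to InteractDistance.
; A hit on itself sets a Temp flag, which feeds an empty branch and is then reset.
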(event EventBeginPlay
  (Input|EnableInput (Game|GetPlayerController 0)))

(event EventActorBeginOverlap
  (params (OtherActor :type Actor%20Object%20Reference)))

(event EventTick
  (params (DeltaSeconds :type Float%20%28single-precision%29)))

(event Input|ActionEvents|InputActionInteract
  (params (Key :type Key%20Structure :default "AnyKey"))
  (bind _returnvalue (Game|GetPlayerCharacter 0))
  (bind (_outlocation _outrotation) (Actor|GetActorEyesViewPoint _returnvalue))
  (:Pressed
    (Utilities|FlowControl|Sequence
      (:then_0
        (bind _outhits (Class|KismetSystemLibrary|LineTraceMultiNEW _outlocation (+ _outlocation (* (Math|Vector|GetForwardVector _outrotation) (Variables|ButtonSetup|GetInteractDistance))) "TraceTypeQuery1" false 0 "Persistent" false))
        (for _index (range 0 (Utilities|Array|Length _outhits))
          (if (== self (.HitActor (Collision|BreakHitResult (Utilities|Array|Get(acopy) _outhits _index))))
            (Variables|Default|SetTemp true)))
        (if (Variables|Default|GetTemp)
          _))
      (:then_1
        (Variables|Default|SetTemp false)))))

(fn ConstructionScript)