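; Container is an architecture prop Blueprint for a shipping-container style mesh with a configurable color, set up entirely in the construction script.
; The color comes from an override or from a red, green or blue choice in a default color array.
; It feeds the "Farbe" parameter of a dynamic M_Container material instance.
; The Closed flag currently has no effect, as both branches assign the closed mesh.
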(event EventBeginPlay)

(event EventActorBeginOverlap
  (params (OtherActor :type Actor%20Object%20Reference)))

(event EventTick
  (params (DeltaSeconds :type Float%20%28single-precision%29)))

(fn ConstructionScript
  (bind _mesh (Variables|Default|GetMesh))
  (if (Variables|ContainerSetup|GetClosed)
    (Components|StaticMesh|SetStaticMesh _mesh "/Game/Assets/Building/Mesh/container_closed.container_closed")
    (else
      (Components|StaticMesh|SetStaticMesh _mesh "/Game/Assets/Building/Mesh/container_closed.container_closed")))
  (if (Variables|ContainerSetup|GetUseColorOverride)
    (Variables|Default|SetFinalColor (Variables|ContainerSetup|GetColorOverride))
    (else
      (switch Utilities|FlowControl|Switch|SwitchonDefaultContainerColor (Variables|ContainerSetup|GetColor)
        (:NewEnumerator0
          (Variables|Default|SetFinalColor (Utilities|Array|Get(acopy) (Variables|Default|GetDefaultColors))))
        (:NewEnumerator1
          (Variables|Default|SetFinalColor (Utilities|Array|Get(acopy) (Variables|Default|GetDefaultColors) 1)))
        (:NewEnumerator2
          (Variables|Default|SetFinalColor (Utilities|Array|Get(acopy) (Variables|Default|GetDefaultColors) 2))))))
  (Utilities|FlowControl|Sequence
    (:then_0
      (bind _returnvalue (Rendering|Material|CreateDynamicMaterialInstance (Variables|Default|GetMesh) 0 "/Game/Assets/Building/OtherGraphicsStuff/Container/M_Container.M_Container" :!class /Script/Engine.PrimitiveComponent))
      (Rendering|Material|SetVectorParameterValue _returnvalue "Farbe" (Variables|Default|GetFinalColor) :!class /Script/Engine.MaterialInstanceDynamic))))