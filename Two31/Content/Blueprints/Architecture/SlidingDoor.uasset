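; Configurable multi-panel sliding door that opens and closes for the player and enemies, with locking and optional item-based unlock.
; The construction script builds panel meshes from the Doors array, which a timeline slides between start and end positions.
; Trigger overlaps track occupancy and drive automatic opening and closing, with enemy overrides.
; Open and Close buffer the requested state, which Tick applies after delays or as interruption flags allow.
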(event OnComponentBeginOverlap(TriggerBox)
  (params (OtherActor :type Actor%20Object%20Reference) (OtherComp :type Primitive%20Component%20Object%20Reference) (OtherBodyIndex :type Integer) (bFromSweep :type Boolean) (SweepResult :type Hit%20Result%20Structure%20%28by%20ref%29))
  (Utilities|Casting|CastToEnemyCharacter OtherActor
    (:then
      (Variables|Default|SetVisitorCount (+ (Variables|Default|GetVisitorCount) 1))
      (if (Variables|DoorSetup|GetIsAutoOpen)
        (Utilities|FlowControl|Sequence :!label _label
          (:then_0
            (CallFunction|Open)))
        (elif (Variables|DoorSetup|GetEnemyAutoOverrideOpen)
          (goto _label))))
    (:CastFailed
      (Variables|Default|SetIsPlayerPresent true)
      (CallFunction|PrintMessage)
      (if (Variables|DoorSetup|GetIsAutoOpen)
        (goto _label)
        (elif (and (Variables|DoorSetup|GetDoRequireItem) (Variables|DoorSetup|GetIsLocked))
          (bind _asbp_player_character (Utilities|Casting|CastToBP_PlayerCharacter (Game|GetPlayerCharacter 0)))
          (if (Class|PlayerCharacter|PlayerHasItem _asbp_player_character (Variables|DoorSetup|GetRequiredItemID))
            (CallFunction|Unlock)))))))

(event OnComponentEndOverlap(TriggerBox)
  (params (OtherActor :type Actor%20Object%20Reference) (OtherComp :type Primitive%20Component%20Object%20Reference) (OtherBodyIndex :type Integer))
  (Utilities|Casting|CastToEnemyCharacter OtherActor
    (:then
      (Variables|Default|SetVisitorCount (+ (Variables|Default|GetVisitorCount) -1)))
    (:CastFailed
      (Variables|Default|SetIsPlayerPresent false)))
  (bind _result (CallFunction|IsEmpty))
  (if _result
    (if (Variables|DoorSetup|GetIsAutoClose)
      (CallFunction|Close false :!label _label)
      (else
        (Utilities|Casting|CastToEnemyCharacter OtherActor)
        (if (Variables|DoorSetup|GetEnemyAutoOverrideClose)
          (goto _label))))))

(event Custom|OnUnlock
  (CallFunction|Open))

(event Custom|OnLock
  (CallFunction|Close false))

(event Custom|CustomEvent_0
  (if (Variables|DoorSetup|GetDoEmptyCheck)
    (CallFunction|Close false)))

(event EventBeginPlay
  (EventDispatchers|BindEventtoOnOpened (delegate Custom|CustomEvent_0)))

(event EventTick
  (params (DeltaSeconds :type Float%20%28single-precision%29))
  (Utilities|FlowControl|Sequence
    (:then_0
      (bind _return (CallFunction|IsMoving))
      (if _return
        (if (Variables|DoorSetup|GetIsOpen)
          (if (Variables|DoorSetup|GetCanInterruptOpening)
            (Variables|DoorSetup|SetIsOpen (Variables|Default|GetIsOpenBuffer) :!label _label))
          (elif (Variables|DoorSetup|GetCanInterruptClosing)
            (goto _label)))
        (elif (<= (Variables|Default|GetDelayTimer) 0.0)
          (goto _label))))
    (:then_1
      (if (Variables|DoorSetup|GetIsOpen)
        (bind _driver (Timeline|Timeline%20DoorDriver Play)
          (:Update
            (bind _output_get (Variables|Default|SetLerpValue _driver))
            (for (_array_element _array_index) (Variables|DoorSetup|GetDoors)
              (Transformation|SetRelativeLocation (Utilities|Array|Get(acopy) (Variables|Default|GetDoorArray) _array_index) (Math|Vector|Lerp(Vector) (.StartingPosition (Utilities|Struct|BreakDoorStruct _array_element)) (.EndPosition (Utilities|Struct|BreakDoorStruct _array_element)) _output_get) false false)))
          (:Finished
            (if (Variables|DoorSetup|GetIsOpen)
              (Default|CallOnOpened)
              (else
                (Default|CallOnClosed)))))
        (else
          (Timeline|Timeline%20DoorDriver Reverse))))
    (:then_2
      (Variables|Default|SetDelayTimer (- (Variables|Default|GetDelayTimer) DeltaSeconds)))))

(fn ConstructionScript
  (Utilities|FlowControl|Sequence
    (:then_0
      (for (_array_element _array_index) (Variables|DoorSetup|GetDoors)
        (bind _returnvalue (AddComponent|AddStaticMeshComponent false))
        (Components|StaticMesh|SetStaticMesh _returnvalue (.Mesh (Utilities|Struct|BreakDoorStruct _array_element)))
        (Transformation|SetRelativeLocation _returnvalue (.StartingPosition (Utilities|Struct|BreakDoorStruct _array_element)) false false)
        (Transformation|SetRelativeRotation _returnvalue (Math|Rotator|MakeRotator (.X (Math|Vector|BreakVector (.Rotation (Utilities|Struct|BreakDoorStruct _array_element)))) (.Y (Math|Vector|BreakVector (.Rotation (Utilities|Struct|BreakDoorStruct _array_element)))) (.Z (Math|Vector|BreakVector (.Rotation (Utilities|Struct|BreakDoorStruct _array_element))))) false false)
        (Utilities|Array|SetArrayElem (Variables|Default|GetDoorArray) _array_index _returnvalue true)))
    (:then_2
      (Transformation|SetRelativeScale3D (Variables|Default|GetTriggerBox) (Variables|DoorSetup|GetTriggerScale)))
    (:then_3
      (Utilities|FlowControl|Sequence
        (:then_0
          (Components|StaticMesh|SetStaticMesh (Variables|Default|GetDoorFrame) (Variables|DoorSetup|GetDoorFrameMesh)))))
    (:then_4
      (Components|Timeline|SetPlayRate (Variables|Default|GetTimeline%20DoorDriver) (/ 1.0 (Variables|DoorSetup|GetAnimationTime))))))

(fn Lock
  (Variables|DoorSetup|SetIsLocked true)
  (CallFunction|OnLock))

(fn Unlock
  (Variables|DoorSetup|SetIsLocked false)
  (CallFunction|OnUnlock))

(fn Close
  (params (AgressiveClose :type Boolean))
  (bind _doorsounds (Variables|Default|GetDoorSounds))
  (if AgressiveClose
    (if (Variables|DoorSetup|GetIsLocked) :!label _label
      (if (Variables|DoorSetup|GetCanCloseLocked)
        (bind _return (CallFunction|IsMoving :!label _label_2))
        (if _return
          _
          (else
            (Variables|Default|SetDelayTimer (Variables|DoorSetup|GetClosingDelay))))
        (Variables|Default|SetIsOpenBuffer false)
        (Variables|Default|SetVisitorCount 0)
        ;[1 1 1] Sound
        (Class|FMODAudioComponent|SetParameter _doorsounds "OpenClosed" 0.0)
        (Class|FMODAudioComponent|Play _doorsounds))
      (else
        (goto _label_2)))
    (else
      (bind _result (CallFunction|IsEmpty))
      (if _result
        (goto _label)))))

(fn Open
  (bind _doorsounds (Variables|Default|GetDoorSounds))
  (Utilities|FlowControl|Sequence
    (:then_0
      (if (Variables|DoorSetup|GetIsLocked)
        (if (Variables|DoorSetup|GetCanOpenLocked)
          (bind _return (CallFunction|IsMoving :!label _label))
          (if _return
            _
            (else
              (Variables|Default|SetDelayTimer (Variables|DoorSetup|GetOpeningDelay))))
          (Variables|Default|SetIsOpenBuffer true)
          ;[1 1 1] Sound
          (Class|FMODAudioComponent|SetParameter _doorsounds "OpenClosed" 1.0)
          (Class|FMODAudioComponent|Play _doorsounds))
        (else
          (goto _label))))))

(fn IsMoving
  (return (not (or (== (Variables|Default|GetLerpValue) 0.0) (== (Variables|Default|GetLerpValue) 1.0)))))

(fn IsEmpty
  (return (and (== (Variables|Default|GetVisitorCount) 0) (not (Variables|Default|GetIsPlayerPresent)))))

(fn PrintMessage
  ;[1 1 1] Locked Door Message
  (bind _asbp_player_character (Utilities|Casting|CastToBP_PlayerCharacter (Game|GetPlayerCharacter 0)))
  (Class|PlayerCharacter|AddDisplayText _asbp_player_character (Variables|DoorSetup|GetDoorLockedText)))