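; BP_SMG is a submachine gun weapon Blueprint that defines how its hits affect the world.
; Every Tick it snaps itself to a fixed relative location and rotation.
; OnWeaponHit applies radius damage with an impulse to Destructible Components, or otherwise spawns a metal decal aligned to the hit normal.
; A debug print of the impact normal remains in the graph but is never executed.
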(event EventOnWeaponHit
  (params (HitResult :type Hit%20Result%20Structure))
  (bind (_bblockinghit _binitialoverlap _time _location _impactpoint _normal _impactnormal _physmat _hitactor _hitcomponent) (Collision|BreakHitResult HitResult))
  (bind _asdestructible_component (Utilities|Casting|CastToDestructibleComponent _hitcomponent)
    (:then
      (Class|DestructibleComponent|ApplyRadiusDamage _asdestructible_component 1.0 _location 1.0 5e+03 false))
    (:CastFailed
      (Rendering|Decal|SpawnDecalatLocation "/Game/Assets/Materials/Decal/BulletHoles/Metal1.Metal1" "50.000000,50.000000,5.000000" _location (Math|Conversions|RotationFromXVector (* _normal -1.0)) 0.0))))

(event EventBeginPlay)

(event EventActorBeginOverlap
  (params (OtherActor :type Actor%20Object%20Reference)))

(event EventTick
  (params (DeltaSeconds :type Float%20%28single-precision%29))
  (Transformation|SetActorRelativeLocation "-35.000000,7.000000,135.000000" false true)
  (Transformation|SetActorRelativeRotation "0.000000,10.000000,0.000000"))

(fn ConstructionScript)