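; Player character Blueprint that adds the HUD and drives movement and pickup audio.
; BeginPlay creates the crosshair and general HUD widgets and narrows the camera manager's pitch limits.
; Tick feeds scaled velocity into the movement sound's isRunning parameter for footsteps.
; PickedUpItem casts by pickup type and sets one parameterised sound's kind before playing it, skipping health or armor sounds when that stat equals 100.
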(event EventBeginPlay
  (bind _returnvalue (Game|GetPlayerCameraManager 0))
  (Utilities|FlowControl|Sequence
    (:then_0
      (bind _returnvalue_2 (UserInterface|CreateWidget "/Game/Blueprints/HUD/WB_Crosshair.WB_Crosshair_C"))
      (UserInterface|Viewport|AddtoViewport _returnvalue_2 0))
    (:then_1
      (bind _returnvalue_3 (UserInterface|CreateWidget "/Game/Blueprints/HUD/WB_GeneralHUD.WB_GeneralHUD_C"))
      (UserInterface|Viewport|AddtoViewport _returnvalue_3 0))
    (:then_2
      ;[1 1 1] Fix Camera Lock
      (Variables|/Script/Engine.PlayerCameraManager|SetViewPitchMax _returnvalue (- (Variables|/Script/Engine.PlayerCameraManager|GetViewPitchMax _returnvalue) 3e+01)))
    (:then_3
      (Variables|/Script/Engine.PlayerCameraManager|SetViewPitchMin _returnvalue (- (Variables|/Script/Engine.PlayerCameraManager|GetViewPitchMin _returnvalue) -3e+01)))))

(event EventPickedUpItem
  (bind _pickup_sound (Variables|Default|GetPickUp%20Sound))
  ;[1 0.006773 0.9628] Pickup sounds
  (bind _aspickup (Utilities|Casting|CastToPickup))
  (Utilities|FlowControl|Sequence
    (:then_0
      (Utilities|Casting|CastToHealthPickup _aspickup)
      (if (not (== (Class|PlayerCharacter|GetHealth) 1e+02))
        (Class|FMODAudioComponent|SetParameter _pickup_sound "kindOfPickUp" 0.0)
        (Class|FMODAudioComponent|Play _pickup_sound)))
    (:then_1
      (Utilities|Casting|CastToArmorPickup _aspickup)
      (if (not (== (Class|PlayerCharacter|GetArmor) 1e+02))
        (Class|FMODAudioComponent|SetParameter _pickup_sound "kindOfPickUp" 1.0)
        (Class|FMODAudioComponent|Play _pickup_sound)))
    (:then_2
      (Utilities|Casting|CastToWeaponPickup _aspickup)
      (Class|FMODAudioComponent|SetParameter _pickup_sound "kindOfPickUp" 2.0)
      (Class|FMODAudioComponent|Play _pickup_sound))))

(event EventTick
  (params (DeltaSeconds :type Float%20%28single-precision%29))
  ;[0.1649 1 0] Footsteps
  (Class|FMODAudioComponent|SetParameter (Variables|Default|GetMovment) "isRunning" (/ (Math|Vector|VectorLength (Variables|/Script/Engine.MovementComponent|GetVelocity (Variables|Character|GetCharacterMovement))) 1e+03)))

(fn ConstructionScript)