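; Enemy spawn area actor that scatters static mesh instances through a box volume; it contains no enemy spawning or runtime logic.
; The construction script sizes the SpawnArea box from AreaExtent, then loops over NumObjects to add InstancedStaticMesh instances at seeded random-stream positions.
; Z spans the full box height, but X and Y range only from zero to the positive extent, covering one quadrant.
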(event EventBeginPlay)

(event EventActorBeginOverlap
  (params (OtherActor :type Actor%20Object%20Reference)))

(event EventTick
  (params (DeltaSeconds :type Float%20%28single-precision%29)))

(fn ConstructionScript
  (bind _spawnarea (Variables|Default|GetSpawnArea))
  (bind _boxextent (Variables|/Script/Engine.BoxComponent|GetBoxExtent _spawnarea))
  (Components|Box|SetBoxExtent _spawnarea (Variables|Default|GetArea%20Extent) true)
  (for _index (range 0 (Variables|Default|GetNumObjects))
    (Components|InstancedStaticMesh|AddInstance (Variables|Default|GetInstancedStaticMesh) (Math|Transform|MakeTransform (Math|Vector|MakeVector (Math|Random|RandomFloatinRangefromStream 0.0 (.x _boxextent) (Variables|Default|GetStream)) (Math|Random|RandomFloatinRangefromStream 0.0 (.y _boxextent) (Variables|Default|GetStream)) (Math|Random|RandomFloatinRangefromStream (* (.z _boxextent) -1.0) (.z _boxextent) (Variables|Default|GetStream))) "0, 0, 0" "1,1,1"))))