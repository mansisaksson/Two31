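; Pickup item Blueprint that sets a keycard colour material and can cue music and ambience changes when the player touches it.
; The construction script picks the blue, red or yellow material from KeycardColour.
; With ShouldPlaySting on, BeginPlay finds the music and ambience actors.
; Player overlap with TriggerSphere then raises the music's Stinger parameter, optionally calls CallPlayAmbience, and delay-stops the BP_Ambience actor.
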(event OnComponentBeginOverlap(TriggerSphere)
  (params (OtherActor :type Actor%20Object%20Reference) (OtherComp :type Primitive%20Component%20Object%20Reference) (OtherBodyIndex :type Integer) (bFromSweep :type Boolean) (SweepResult :type Hit%20Result%20Structure%20%28by%20ref%29))
  ;[1 1 1] StingerBollen
  (if (Variables|Default|GetShouldPlaySting)
    (Utilities|Casting|CastToPlayerCharacter OtherActor)
    (Class|FMODAudioComponent|SetParameter (Variables|/Game/Blueprints/Music/BP_MusicActor.BP_MusicActor_C|GetMusic (Variables|Default|GetMusicActor)) "Stinger" 1.0)
    (Utilities|FlowControl|Sequence
      (:then_0
        (if (Variables|Default|GetAmbience)
          (Default|CallPlayAmbience)))
      (:then_1
        (Default|DelayedStop (Variables|Default|GetBP_Ambience) 2.0)))))

(event EventBeginPlay
  (if (Variables|Default|GetShouldPlaySting)
    (bind _outactors (Actor|GetAllActorsOfClass "/Game/Blueprints/Music/BP_MusicActor.BP_MusicActor_C"))
    (Variables|Default|SetMusicActor (Utilities|Array|Get(acopy) _outactors))
    (bind _outactors_2 (Actor|GetAllActorsOfClass "/Game/Blueprints/Music/BP_Ambience.BP_Ambience_C"))
    (Variables|Default|SetBP_Ambience (Utilities|Array|Get(acopy) _outactors_2))))

(fn ConstructionScript
  (switch Utilities|FlowControl|Switch|SwitchonKeycardColour (Variables|Default|GetKeycard%20Colour)
    (:NewEnumerator0
      (Rendering|Material|SetMaterial (Variables|Default|GetItemMesh) 0 "/Game/Assets/Building/OtherGraphicsStuff/Pickups/Keycard/M_KeycardBlue.M_KeycardBlue"))
    (:NewEnumerator1
      (Rendering|Material|SetMaterial (Variables|Default|GetItemMesh) 0 "/Game/Assets/Building/OtherGraphicsStuff/Pickups/Keycard/M_KeycardRed.M_KeycardRed"))
    (:NewEnumerator2
      (Rendering|Material|SetMaterial (Variables|Default|GetItemMesh) 0 "/Game/Assets/Building/OtherGraphicsStuff/Pickups/Keycard/M_KeycardYellow.M_KeycardYellow"))))