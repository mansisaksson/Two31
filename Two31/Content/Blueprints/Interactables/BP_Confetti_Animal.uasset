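; Interactable animal prop that spawns a particle effect, presumably confetti, when it takes any damage, then destroys itself after a delay.
; The construction script picks a giraffe or elephant mesh from the AnimalType variable and nudges ParticleOrigin to suit each elephant variant.
; The damage event has no guard, so repeated hits before destruction can spawn additional effects.
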(event EventBeginPlay)

(event EventActorBeginOverlap
  (params (OtherActor :type Actor%20Object%20Reference)))

(event EventTick
  (params (DeltaSeconds :type Float%20%28single-precision%29)))

(event Game|Damage|EventAnyDamage
  (params (Damage :type Float%20%28single-precision%29) (DamageType :type Damage%20Type%20Object%20Reference) (InstigatedBy :type Controller%20Object%20Reference) (DamageCauser :type Actor%20Object%20Reference))
  (bind _returnvalue (Effects|SpawnEmitteratLocation (Variables|ConfettiSetup|GetParticleEffect) (Transformation|GetWorldLocation (Variables|Default|GetParticleOrigin))))
  (Transformation|SetWorldScale3D _returnvalue "1.000000,1.000000,1.000000")
  (Utilities|FlowControl|Delay (Variables|ConfettiSetup|GetDestroyDelay))
  (Actor|DestroyActor))

(fn ConstructionScript
  (switch Utilities|FlowControl|Switch|SwitchonAnimalTypes (Variables|ConfettiSetup|GetAnimalType)
    (:NewEnumerator0
      (Components|StaticMesh|SetStaticMesh (Variables|Default|GetAnimal) "/Game/Assets/Special/Mesh_giraffe_1.Mesh_giraffe_1"))
    (:NewEnumerator1
      (Components|StaticMesh|SetStaticMesh (Variables|Default|GetAnimal) "/Game/Assets/Special/Mesh_LargeElephant_1.Mesh_LargeElephant_1")
      (Transformation|AddRelativeLocation (Variables|Default|GetParticleOrigin) "0, 0,72.000000" false false))
    (:NewEnumerator2
      (Components|StaticMesh|SetStaticMesh (Variables|Default|GetAnimal) "/Game/Assets/Special/Mesh_ScaryElephant_1.Mesh_ScaryElephant_1")
      (Transformation|AddRelativeLocation (Variables|Default|GetParticleOrigin) "-8.000000, 0,72.000000" false false))
    (:NewEnumerator3
      (Components|StaticMesh|SetStaticMesh (Variables|Default|GetAnimal) "/Game/Assets/Special/Mesh_SmallElephant_1.Mesh_SmallElephant_1")
      (Transformation|AddRelativeLocation (Variables|Default|GetParticleOrigin) "2.000000, 0,0.000000" false false))))