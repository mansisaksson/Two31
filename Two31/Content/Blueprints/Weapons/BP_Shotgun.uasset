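; BP_Shotgun is a shotgun weapon Blueprint that handles sound, camera shake and attachments.
; On Tick while visible, it plays the reload sound once per reload, shows the flashlight and laser spot, and line-traces from an Arrow to place the spot just short of the hit.
; When hidden, it hides both attachments and stops the reload sound.
; OnBeginFire passes the clip ammo count to the shot sound and shakes the camera.
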(event EventBeginPlay)

(event EventActorBeginOverlap
  (params (OtherActor :type Actor%20Object%20Reference)))

(event EventTick
  (params (DeltaSeconds :type Float%20%28single-precision%29))
  (bind _arrow (Variables|Default|GetArrow))
  (bind _shotgun_reload (Variables|Default|GetShotGun%20Reload))
  (bind _returnvalue (Transformation|GetWorldLocation _arrow))
  (if (not (Variables|Default|GetbHidden))
    (Utilities|FlowControl|Sequence
      (:then_0
        ;[0.9181 0 1] Reload Sound
        (Utilities|FlowControl|Sequence
          (:then_0
            (if (|CanPlaySound)
              (Class|FMODAudioComponent|SetParameter _shotgun_reload "SelectedAnim" 3.0)
              (Class|FMODAudioComponent|Play _shotgun_reload)
              (Variables|Default|SetHasPlayedReloadSound true)))
          (:then_1
            (if (== (Class|Weapon|GetTimeSinceReload) 0.0)
              (Variables|Default|SetHasPlayedReloadSound false)))))
      (:then_1
        ;[1 0 0.02604] Laser Sight
        (CallFunction|SetWeaponAttachmentsHidden false)
        (bind _outhit (Collision|LineTraceForObjects _returnvalue (+ _returnvalue (* (Math|Vector|GetForwardVector _arrow) 5e+03)) (Utilities|Array|MakeArray "ObjectTypeQuery1" "ObjectTypeQuery2" "ObjectTypeQuery4" "ObjectTypeQuery3" "ObjectTypeQuery6") true (Utilities|Array|MakeArray (Class|Weapon|GetOwner)) "None"))
        (Transformation|SetWorldLocation (Variables|Default|GetLaser%20Spot) (- (.Location (Collision|BreakHitResult _outhit)) (* (Math|Vector|GetForwardVector (Variables|Default|GetArrow)) 5e+01)) false true)))
    (else
      ;[0 0.07825 1] Hide Weapon/Stop Weapon Sounds
      (CallFunction|SetWeaponAttachmentsHidden true)
      (bind _returnvalue_2 (Class|FMODAudioComponent|IsPlaying (Variables|Default|GetShotGun%20Reload)))
      (if _returnvalue_2
        (Class|FMODAudioComponent|Stop (Variables|Default|GetShotGun%20Reload))))))

(event EventOnBeginFire
  (bind _shotgun_sound (Variables|Default|GetShotGun%20Sound))
  ;[0.8697 0 1] Fire Sound
  (if (not (Variables|Default|GetbHidden))
    (if (Class|Weapon|GetCanFire)
      (Class|FMODAudioComponent|SetParameter _shotgun_sound "Ammo" (Math|Conversions|ToFloat(Integer) (Class|Weapon|GetAmmoinClip)))
      (Class|FMODAudioComponent|Play _shotgun_sound)
      ;[1 0.108 0.4002] Camera Shake
      (Class|PlayerController|ClientPlayCameraShake (Game|GetPlayerController 0) "/Game/Blueprints/BP_CameraShake.BP_CameraShake_C" 1.0 "CameraLocal" "0, 0, 0"))))

(fn ConstructionScript
  (Class|SceneComponent|Attachto (Variables|Default|GetLazer) (Variables|Default|GetWeaponMesh) "LaserSight" "KeepRelativeOffset" true))

(fn SetWeaponAttachmentsHidden
  (params (Hidden%20In%20Game :type Boolean))
  (bind _returnvalue (not Hidden%20In%20Game))
  (Rendering|SetVisibility (Variables|Default|GetLaser%20Spot) _returnvalue false)
  (Rendering|SetVisibility (Variables|Default|GetFlash%20Light) _returnvalue false))